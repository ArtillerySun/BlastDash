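; BP_NPCManager tracks how many NPCs are alive in the level and triggers the win when none remain.
; On BeginPlay it registers every placed BP_NPC, incrementing the count and notifying BP_FirstPersonGameMode of each spawn.
; UnregisterNPC decrements the count, clamped at zero, then calls Win once when it reaches zero, otherwise reporting the death to the game mode.
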(event EventBeginPlay
  (bind _outactors (Actor|GetAllActorsOfClass "/Game/AI/BP_NPC.BP_NPC_C"))
  (for _array_element _outactors
    (CallFunction|RegisterNPC)))

(event Collision|EventActorBeginOverlap
  (params (OtherActor :type Actor%20Object%20Reference)))

(event EventTick
  (params (DeltaSeconds :type Float%20%28single-precision%29)))

(fn ConstructionScript)

(fn RegisterNPC
  (Variables|Default|SetAliveNPCCount (+ (Variables|Default|GetAliveNPCCount) 1))
  (bind _asbp_first_person_game_mode (Utilities|Casting|CastToBP_FirstPersonGameMode (Game|GetGameMode)))
  (Default|NPCSpawned _asbp_first_person_game_mode))

(fn UnregisterNPC
  (bind _returnvalue (Game|GetGameMode))
  (bind _output_get (Variables|Default|SetAliveNPCCount (Math|Integer|Max(Integer) 0 (- (Variables|Default|GetAliveNPCCount) 1))))
  (if (and (== _output_get 0) (not (Variables|Default|GetGameWon)))
    (Variables|Default|SetGameWon true)
    (bind _asbp_first_person_game_mode (Utilities|Casting|CastToBP_FirstPersonGameMode _returnvalue))
    (Default|Win _asbp_first_person_game_mode)
    (else
      (bind _asbp_first_person_game_mode_2 (Utilities|Casting|CastToBP_FirstPersonGameMode _returnvalue))
      (Default|NPCDied _asbp_first_person_game_mode_2))))