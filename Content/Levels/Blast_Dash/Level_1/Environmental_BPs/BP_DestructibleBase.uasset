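; Base destructible environment actor that takes damage, shatters into Chaos debris and respawns after a delay.
; Damage drives a dynamic material overlay; at zero health it swaps the static mesh for a Geometry Collection, applying strain and radial impulse from the damage causer's location.
; Debris collisions deal velocity-scaled, timer-gated damage to the player and other destructibles.
; After despawning debris, it spawns a fresh copy at its original transform and destroys itself.
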(event OnChaosPhysicsCollision(GeometryCollection)
  (params (CollisionInfo :type Chaos%20Physics%20Collision%20Info%20Structure%20%28by%20ref%29))
  (bind (_component _othercomponent _location _normal _accumulatedimpulse _velocity _othervelocity) (Utilities|Struct|BreakChaosPhysicsCollisionInfo CollisionInfo))
  (bind _debrismindamagespeed (Variables|Default|GetDebrisMinDamageSpeed))
  (bind _returnvalue (Components|GetOwner _othercomponent))
  (bind _returnvalue_2 (- _velocity _othervelocity))
  (bind _returnvalue_3 (Math|Vector|VectorLength _returnvalue_2))
  (bind _returnvalue_4 (- _returnvalue_3 _debrismindamagespeed))
  (bind _returnvalue_5 (* _returnvalue_4 0.05))
  ;[0.15 0.15 0.15 0.5] Debris Damage
  (if (not (== _returnvalue self))
    (bind _asbp_first_person_character (Utilities|Casting|CastToBP_FirstPersonCharacter _returnvalue)
      (:then
        (if (>= _returnvalue_3 _debrismindamagespeed)
          (Utilities|FlowControl|DoOnce false
            (:Completed
              (Game|Damage|ApplyDamage _asbp_first_person_character _returnvalue_5 0 0)
              (Utilities|Time|SetTimerbyEvent (delegate Custom|ResetDamageGatePlayer) 0.2)))))
      (:CastFailed
        (bind _asbp_destructible_base (Utilities|Casting|CastToBP_DestructibleBase _returnvalue))
        (Utilities|FlowControl|DoOnce false
          (:Completed
            (Game|Damage|ApplyDamage _asbp_destructible_base _returnvalue_5 0 0)
            (Utilities|Time|SetTimerbyEvent (delegate Custom|ResetDamageGateTerrain) 0.4)))))))

(event Custom|ResetDamageGatePlayer
  ;[0.15 0.15 0.15 0.5] Debris Damage
  (Utilities|FlowControl|DoOnce false) ; enters at Reset
)

(event Custom|ResetDamageGateTerrain
  ;[0.15 0.15 0.15 0.5] Debris Damage
  (Utilities|FlowControl|DoOnce false) ; enters at Reset
)

(event EventBeginPlay
  (Variables|Default|SetOriginalTransform (Transformation|GetActorTransform))
  (Variables|Default|SetInitialHealth (Variables|Default|GetCurrHealth))
  (bind _returnvalue (Rendering|Material|CreateDynamicMaterialInstance (Variables|Default|GetStaticMesh) 0 "/Game/Materials/Solids/MI_Solid_Red.MI_Solid_Red" "None" :!class /Script/Engine.PrimitiveComponent))
  (Variables|Default|SetDamageMatRef _returnvalue))

(event Collision|EventActorBeginOverlap
  (params (OtherActor :type Actor%20Object%20Reference)))

(event EventTick
  (params (DeltaSeconds :type Float%20%28single-precision%29)))

(event Game|Damage|EventAnyDamage
  (params (Damage :type Float%20%28single-precision%29) (DamageType :type Damage%20Type%20Object%20Reference) (InstigatedBy :type Controller%20Object%20Reference) (DamageCauser :type Actor%20Object%20Reference))
  ;[0.15 0.15 0.15 0.5] Health Calculation + Broken check
  (if (not (Variables|Default|GetbBroken))
    (bind _output_get (Variables|Default|SetCurrHealth (- (Variables|Default|GetCurrHealth) Damage)))
    (if (Utilities|IsValid DamageCauser)
      (Variables|Default|SetLastExplosionOrigin (Transformation|GetActorLocation DamageCauser))
      (else
        (Variables|Default|SetLastExplosionOrigin (Transformation|GetActorLocation))))
    ;[0.15 0.15 0.15 0.5] Texture Overlay
    (Rendering|Material|SetScalarParameterValue (Variables|Default|GetDamageMatRef) "DamageAmount" (* (- 1.0 (/ (Variables|Default|GetCurrHealth) (Variables|Default|GetInitialHealth))) 2.0) :!class /Script/Engine.MaterialInstanceDynamic)
    ;[0.15 0.15 0.15 0.5] Break and Respawn
    (if (<= _output_get 0.0)
      (CallFunction|BreakfromExplosion (Variables|Default|GetLastExplosionOrigin))
      (Utilities|FlowControl|Delay (Variables|Default|GetDespawnTimer))
      (CallFunction|DespawnBrokenPieces)
      (Utilities|FlowControl|Delay (Variables|Default|GetRespawnDelay))
      (CallFunction|RespawnDestructible))))

(fn ConstructionScript)

(fn BreakfromExplosion
  (params (ExplosionOrigin :type Vector))
  (bind _staticmesh (Variables|Default|GetStaticMesh))
  (bind _breakradius (Variables|Default|GetBreakRadius))
  (bind _geometrycollection (Variables|Default|GetGeometryCollection))
  (if (not (Variables|Default|GetbBroken))
    (Variables|Default|SetbBroken true)
    (Variables|Default|SetLastExplosionOrigin ExplosionOrigin)
    (Rendering|SetVisibility _staticmesh false false)
    (Collision|SetCollisionEnabled _staticmesh "NoCollision")
    (Rendering|SetVisibility _geometrycollection true false)
    (Collision|SetCollisionEnabled _geometrycollection "QueryAndPhysics")
    (Class|GeometryCollectionComponent|ApplyExternalStrain _geometrycollection 0 (Variables|Default|GetLastExplosionOrigin) _breakradius (Variables|Default|GetPropagationDepth) (Variables|Default|GetPropagationFactor) (Variables|Default|GetBreakStrain))
    (Physics|AddRadialImpulse _geometrycollection (Variables|Default|GetLastExplosionOrigin) _breakradius (Variables|Default|GetBreakImpulseStrength) "RIF_Linear" true)))

(fn DespawnBrokenPieces
  (bind _geometrycollection (Variables|Default|GetGeometryCollection))
  (Rendering|SetVisibility _geometrycollection false false)
  (Collision|SetCollisionEnabled _geometrycollection "NoCollision")
  (Physics|SetSimulatePhysics _geometrycollection false))

(fn RespawnDestructible
  (bind _self self)
  (bind _returnvalue (Utilities|GetClass _self))
  (bind (_bbroken _currhealth _breakradius _breakimpulsestrength _breakstrain _propagationdepth _propagationfactor) (Utilities|GetClassDefaults _returnvalue))
  (Game|SpawnActorfromClass _returnvalue (Variables|Default|GetOriginalTransform) "Undefined" "MultiplyWithRoot" 0 (Variables|Default|GetInitialHealth) _breakradius _breakimpulsestrength _breakstrain _propagationdepth _propagationfactor 0)
  (Actor|DestroyActor))