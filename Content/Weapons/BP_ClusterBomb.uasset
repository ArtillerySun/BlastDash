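; BP_ClusterBomb is a bomb that releases a set of child bombs after a delay.
; On BeginPlay it activates, sets its explosion radius and force, then waits for the explosion delay time.
; It then spawns one configurable bomb class per Offset entry, 100 units from itself.
; Each spawn direction comes from the actor's rotation combined with an axes-built rotation whose Up vector alone scales with that entry.
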(event EventBeginPlay
  (Class|BDProjectile|ActivateBomb)
  (Variables|Default|SetExplosionRadius 3e+02)
  (Variables|Default|SetExplosionForce 1e+03)
  (bind _returnvalue (Class|BDProjectile|GetExplosionDelayTime))
  (Utilities|FlowControl|Delay _returnvalue)
  (for _array_element (Variables|Default|GetOffset)
    (Game|SpawnActorfromClass (Variables|Default|GetBombClassToSpawn) (Math|Transform|MakeTransform (Math|Transform|TransformLocation (Math|Transform|MakeTransform (Transformation|GetActorLocation) (Math|Transform|TransformRotation (Transformation|GetActorTransform) (Math|Rotator|MakeRotationfromAxes "0, 0, 0" "0, 0, 0" (* _array_element "45.000000,0.000000,0.000000")))) "100.000000,0.000000,0.000000")) "Undefined" "MultiplyWithRoot" 0 0)))

(event Collision|EventActorBeginOverlap
  (params (OtherActor :type Actor%20Object%20Reference)))

(event EventTick
  (params (DeltaSeconds :type Float%20%28single-precision%29)))

(fn ConstructionScript)