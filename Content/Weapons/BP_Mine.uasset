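; BP_Mine is a throwable proximity mine that sticks where it first hits after being thrown, then explodes when triggered.
; It builds on a parent explosive projectile, setting a very long fuse, zeroing velocity and gravity on impact, and ignoring further hold changes once released.
; A sphere overlap on the deployed, non-hovering mine plays an alert and, after a delay, shortens the fuse.
; Early detonation is overridden empty; explosion effects spawn particles and sound.
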(event OnComponentBeginOverlap(Sphere)
  (params (OverlappedComponent :type Primitive%20Component%20Object%20Reference) (OtherActor :type Actor%20Object%20Reference) (OtherComp :type Primitive%20Component%20Object%20Reference) (OtherBodyIndex :type Integer) (bFromSweep :type Boolean) (SweepResult :type Hit%20Result%20Structure%20%28by%20ref%29))
  (if (not (Variables|Default|GetbIsHovering))
    (if (Variables|Default|GetbIsDeployed)
      (Audio|PlaySoundatLocation "/Game/Audio/SoundWaves/Effect/SW_Alert.SW_Alert" "0, 0, 0" "0, 0, 0" 1.0 1.0 0.0 0 0 0 0)
      (Utilities|FlowControl|Delay 1.0)
      (Class|BDProjectile|SetExplosionDelayTime 0.5))))

(event EventBeginPlay
  (Class|BDProjectile|SetExplosionDelayTime 9999.0)
  (Variables|Default|SetbIsDeployed false)
  (Variables|Default|SetbWasThrown false))

(event EventSetHeld
  (params (bHeld :type Boolean))
  (if (not (Variables|Default|GetbWasThrown))
    (if bHeld
      _
      (else
        (Variables|Default|SetbWasThrown true)))
    (|CallParentFunction bHeld)))

(event EventTriggerEarlyDetonation)

(event EventOnExplosionEffects
  (bind _self self)
  (bind _returnvalue (Transformation|GetActorLocation _self))
  (Effects|SpawnEmitteratLocation "/Game/Effects/Particles/Explosion/P_AsteroidExplosion.P_AsteroidExplosion" _returnvalue)
  (Audio|PlaySoundatLocation "/Game/Audio/SoundWaves/Effect/SW_Explosion_1.SW_Explosion_1" _returnvalue "0, 0, 0" 1.0 1.0 0.0 0 0 0 0))

(event EventOnProjectileImpact
  (params (Hit :type Hit%20Result%20Structure%20%28by%20ref%29))
  (if (Variables|Default|GetbWasThrown)
    (if (not (Variables|Default|GetbIsDeployed))
      (Variables|Default|SetbIsDeployed true)
      (Variables|Default|SetVelocity "0, 0, 0")
      (Variables|Default|SetGravity "0, 0, 0"))))

(fn ConstructionScript)