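; Gravity bomb weapon that yanks nearby pawns and physics bodies toward itself before exploding.
; A sphere overlap applies a one-shot inward velocity through the physics-interactable interface, falling back to launching characters or adding impulses to simulating root components.
; After a short delay it runs the parent class's explosion, whose radius and force are set on BeginPlay alongside the gravity values.
; It overrides the effects event with its own particle and sound.
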(event EventBeginPlay
  (Variables|Default|SetExplosionRadius 5e+02)
  (Variables|Default|SetExplosionForce 8e+03)
  (Variables|Default|SetGravityForce 2e+03)
  (Variables|Default|SetGravityRadius 1e+03))

(event Collision|EventActorBeginOverlap
  (params (OtherActor :type Actor%20Object%20Reference)))

(event EventTick
  (params (DeltaSeconds :type Float%20%28single-precision%29)))

(event EventOnExplosionEffects
  (bind _self self)
  (bind _returnvalue (Transformation|GetActorLocation _self))
  (Effects|SpawnEmitteratLocation "/Game/Effects/Particles/Explosion/P_AsteroidExplosion.P_AsteroidExplosion" _returnvalue)
  (Audio|PlaySoundatLocation "/Game/Audio/SoundWaves/Effect/SW_Explosion_1.SW_Explosion_1" _returnvalue "0, 0, 0" 1.0 1.0 0.0 0 0 0 0))

(event EventExecuteExplosion
  (bind _outactors (Collision|SphereOverlapActors (Transformation|GetActorLocation) (Variables|Default|GetGravityRadius) (Utilities|Array|MakeArray "ObjectTypeQuery3" "ObjectTypeQuery4") 0))
  (for _array_element _outactors
    (if (Utilities|DoesObjectImplementInterface _array_element "/Script/BlastDash.BD_PhysicsInteractable")
      (Class|BDPhysicsInteractable|ApplyCustomImpulse(Message) _array_element (* (Math|Vector|Normalize (- (Transformation|GetActorLocation) (Transformation|GetActorLocation _array_element))) (Variables|Default|GetGravityForce)) true)
      (else
        (bind _ascharacter (Utilities|Casting|CastToCharacter _array_element)
          (:then
            (Character|LaunchCharacter _ascharacter (* (Math|Vector|Normalize (- (Transformation|GetActorLocation) (Transformation|GetActorLocation _array_element))) (Variables|Default|GetGravityForce)) false false))
          (:CastFailed
            (bind _asprimitive_component (Utilities|Casting|CastToPrimitiveComponent (Variables|/Script/Engine.Actor|GetRootComponent _array_element)))
            (if (Physics|IsSimulatingPhysics _asprimitive_component "None")
              (Physics|AddImpulse _asprimitive_component (* (Math|Vector|Normalize (- (Transformation|GetActorLocation) (Transformation|GetActorLocation _array_element))) (Variables|Default|GetGravityForce)) "None" true)))))))
  (Utilities|FlowControl|Delay 1.0)
  (|CallParentFunction))

(fn ConstructionScript)